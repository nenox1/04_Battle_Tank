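; Player-controllable tank Blueprint that wires up its components and maps input to driving, camera aiming and firing.
; BeginPlay passes the barrel and turret to their reference setters and initialises TankMovement with both tracks.
; Driving input either sets each track's throttle directly or sends move and turn intents to TankMovement.
; Aim input rotates an azimuth gimbal for yaw and the spring arm for pitch separately, scaled by delta time.
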(event `self.ReceiveBeginPlay`
  (`self.SetBarrelReference` (`self.Barrel`))
  (`self.SetTurretReference` (`self.Turret`))
  (`TankMovementComponent.Initialise` (`self.TankMovement`) (`self.Left Tank Track `) (`self.Right TankTrack`)))

(event `InputAxis|AimAzimuth`
  (params (AxisValue :type "Float (single-precision)"))
  ;[1 1 1] Input binding
  (`SceneComponent.K2_AddLocalRotation` (`self.Azimuth Gimbal`) (`KismetMathLibrary.MakeRotator` 0.0 0.0 (* AxisValue (`GameplayStatics.GetWorldDeltaSeconds`) 100.0)) false false))

(event `InputAxis|Input Left Track`
  (params (AxisValue :type "Float (single-precision)"))
  ;[1 1 1] Movement input binding
  (`TankTrack.SetThrottle` (`self.Left Tank Track `) AxisValue))

(event `InputAxis|Input Right Track`
  (params (AxisValue :type "Float (single-precision)"))
  ;[1 1 1] Movement input binding
  (`TankTrack.SetThrottle` (`self.Right TankTrack`) AxisValue))

(event `InputAxis|AimElevation`
  (params (AxisValue :type "Float (single-precision)"))
  ;[1 1 1] Input binding
  (`SceneComponent.K2_AddLocalRotation` (`self.SpringArm`) (`KismetMathLibrary.MakeRotator` 0.0 (* AxisValue (`GameplayStatics.GetWorldDeltaSeconds`) 100.0)) false false))

(event `InputAxis|Move Foward`
  (params (AxisValue :type "Float (single-precision)"))
  ;[1 1 1] Movement input binding
  (`TankMovementComponent.IntendMoveForward` (`self.TankMovement`) AxisValue))

(event `InputAction|Fire`
  (params (Key :type "Key Structure"))
  ;[1 1 1] Input binding
  (:`Pressed`
    (`self.Fire`)))

(event `InputAxis|Turn Right`
  (params (AxisValue :type "Float (single-precision)"))
  ;[1 1 1] Movement input binding
  (`TankMovementComponent.IntendTurnRight` (`self.TankMovement`) AxisValue))

(event `InputAxis|Turn Left`
  (params (AxisValue :type "Float (single-precision)"))
  ;[1 1 1] Movement input binding
  (`TankMovementComponent.IntendTurnLeft` (`self.TankMovement`) AxisValue))

(fn `UserConstructionScript`)